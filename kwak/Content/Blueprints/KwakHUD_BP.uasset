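; KwakHUD_BP is the Kwak game's HUD, which puts the player's UMG widgets on screen.
; BeginPlay adds the crosshair, and when the owning controller has authority it also adds the Startgame widget and prints the game mode's match state.
; Two custom events show and hide the scoreboard by creating a new widget on each show, storing it, and removing it from its parent on hide.
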(event Custom|showScoreboard
  (bind _returnvalue (UserInterface|CreateWidget "/Game/Blueprints/scoreboard.scoreboard_C" (Game|Player|GetOwningPlayerController)))
  (Variables|Default|Setscoreboard _returnvalue)
  (UserInterface|Viewport|AddtoViewport _returnvalue 0))

(event Custom|HideScoreboard
  (Widget|RemovefromParent (Variables|Default|Getscoreboard)))

(event EventBeginPlay
  (bind _returnvalue (UserInterface|CreateWidget "/Game/Blueprints/KwakCrosshair.KwakCrosshair_C"))
  (UserInterface|Viewport|AddtoViewport _returnvalue 100)
  (if (Ability|HasAuthority (Game|Player|GetOwningPlayerController))
    (bind _returnvalue_2 (UserInterface|CreateWidget "/Game/Blueprints/startgame.startgame_C"))
    (UserInterface|Viewport|AddtoViewport _returnvalue_2 0)
    (Development|PrintString (Utilities|String|ToString(Name) (Class|GameMode|GetMatchState (.AsKwak%20Game%20Mode%20Base%20BP (Utilities|Casting|CastTokwakGameModeBase_BP (Game|GetGameMode))))))))

(event Collision|EventActorBeginOverlap
  (params (OtherActor :type Actor%20Object%20Reference)))

(event EventTick
  (params (DeltaSeconds :type Float%20%28single-precision%29)))

(fn ConstructionScript)